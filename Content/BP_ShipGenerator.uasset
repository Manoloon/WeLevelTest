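; BP_ShipGenerator spawns a square grid of BP_Ship actors when play begins.
; Two nested loops over NumberOfShips create that many ships per side, spaced at fixed intervals in X and Y.
; Grid X and Y are offset from the world origin, while height comes from the generator's own location.
; Each ship receives the generator's Target value at spawn.
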(event `self.ReceiveBeginPlay`
  (bind (_returnvalue_x _returnvalue_y _returnvalue_z) (`KismetMathLibrary.BreakVector` (`self.K2_GetActorLocation`)))
  (bind _numberofships (`self.NumberOfShips`))
  (for _index (range 1 (+ _numberofships 1))
    (for _index_2 (range 1 (+ _numberofships 1))
      (`|SpawnActorFromClass` "/Game/BP_Ship.BP_Ship_C" (`KismetMathLibrary.MakeTransform` (`KismetMathLibrary.MakeVector` (`KismetMathLibrary.Conv_IntToDouble` (* (- _index 2) 200)) (`KismetMathLibrary.Conv_IntToDouble` (* (- _index_2 2) 200)) _returnvalue_z)) "Undefined" "OverrideRootScale" null (`self.Target`) null))))

(fn `UserConstructionScript`)